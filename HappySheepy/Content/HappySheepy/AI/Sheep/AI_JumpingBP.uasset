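; AI controller for jumping sheep that steers them toward the AI_TargetBP actor in the level.
; On BeginPlay it sets up the AI_Jumping_BB blackboard, seeds MoveLocation and runs the AI_JumpingBT behavior tree.
; Every Tick it looks up all target actors again and sets MoveLocation to a random reachable point within a small radius of the first one found.
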(event EventBeginPlay
  (bind _blackboardcomponent (Class|AIController|UseBlackboard "/Game/HappySheepy/AI/Sheep/AI_Jumping_BB.AI_Jumping_BB"))
  (Variables|Default|SetCurrentBlackBoard _blackboardcomponent)
  (bind _outactors (Actor|GetAllActorsOfClass "/Game/HappySheepy/AI/Sheep/AI_TargetBP.AI_TargetBP_C"))
  (AI|Components|Blackboard|SetValueasVector (Variables|Default|GetCurrentBlackBoard) (Utilities|Name|MakeLiteralName "MoveLocation") (.RandomLocation (AI|Navigation|GetRandomReachablePointinRadius (Transformation|GetActorLocation (Utilities|Array|Get(acopy) _outactors)) 25.0 0 0)))
  (AI|RunBehaviorTree "/Game/HappySheepy/AI/Sheep/AI_JumpingBT.AI_JumpingBT"))

(event EventTick
  (params (DeltaSeconds :type Float%20%28single-precision%29))
  (bind _outactors (Actor|GetAllActorsOfClass "/Game/HappySheepy/AI/Sheep/AI_TargetBP.AI_TargetBP_C"))
  (AI|Components|Blackboard|SetValueasVector (Variables|Default|GetCurrentBlackBoard) (Utilities|Name|MakeLiteralName "MoveLocation") (.RandomLocation (AI|Navigation|GetRandomReachablePointinRadius (Transformation|GetActorLocation (Utilities|Array|Get(acopy) _outactors)) 25.0 0 0))))

(fn ConstructionScript)